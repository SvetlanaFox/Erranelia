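; BP_Inventory is the player-facing inventory that stores item slots and owns their UI widget.
; On BeginPlay it sizes the slot array only for a new game, then in either start mode creates the hidden widget on the main HUD canvas, positioned at half the viewport size.
; Each slot holds an item class and amount, with item details read from class defaults.
; GetSaveData packs slot count and contents into a save struct.
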(event EventBeginPlay
  (switch Utilities|FlowControl|Switch|SwitchonE_InventoryStartMode (Variables|Default|GetStartMode)
    (:NewEnumerator0
      (Utilities|Array|Resize (Variables|Default|GetSlots) (Variables|Default|GetAmountOfSlots))
      (CallFunction|CreateInventoryWidget))
    (:NewEnumerator1
      (CallFunction|CreateInventoryWidget))))

(fn ConstructionScript)

(fn GetSaveData
  (return (Utilities|Struct|MakeS_SaveInventoryInfo (Variables|Default|GetAmountOfSlots) (Variables|Default|GetSlots))))

(fn GetSlotInfofromIndex
  (params (Index :type Integer))
  (bind _slots (Variables|Default|GetSlots))
  (bind _output (Utilities|Array|Get(acopy) _slots Index))
  (bind (_item _amount) (Utilities|Struct|BreakS_SlotSignature _output))
  (if (Utilities|IsValidClass _item)
    ;[1 1 1] Слот не пустой
    (return false (Utilities|GetClassDefaults _item) _amount)
    (else
      ;[1 1 1] Слот пустой
      (return true "" 0))))

(fn CreateInventoryWidget
  (bind _returnvalue (Viewport|GetViewportSize))
  ;[1 1 1] Создаем виджет инвентаря и записываем его в переменную
  (bind _returnvalue_2 (UserInterface|CreateWidget "/Game/MyContent/Inventory/Widgets/InventoryWB.InventoryWB_C" 0 self))
  (bind _output_get (Variables|Default|SetInventoryWBRef _returnvalue_2))
  ;[1 1 1] Скрываем инвентарь
  (Widget|SetVisibility _output_get "Hidden")
  ;[1 1 1] Добавляем инвентарь на экран
  (bind _returnvalue_3 (Class|CanvasPanel|AddChildtoCanvas (Variables|/Game/MyContent/UIX/Main_HUD.Main_HUD_C|GetCanvasPanel_0 (Variables|Default|GetMainHudReference)) _output_get))
  (Class|CanvasPanelSlot|SetAutoSize _returnvalue_3 true)
  (Class|CanvasPanelSlot|SetPosition _returnvalue_3 (Math|Vector2D|MakeVector2D (/ (.x _returnvalue) 2.0) (/ (.y _returnvalue) 2.0)))
  (return))